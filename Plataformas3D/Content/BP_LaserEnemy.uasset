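; BP_LaserEnemy is an enemy that fires lasers at intervals while the player character is nearby and dies when shot enough times.
; The player entering DetectionArea starts a looping timer that spawns pooled lasers at LaserPoint; the actor-level end overlap clears it.
; Bullets overlapping EnemyArea return to their pool and remove a life, destroying the enemy when none remain.
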(event `OnEnemyBeginOverlap`
  (params (OverlappedComponent :type "PrimitiveComponent Object Reference") (OtherActor :type "Actor Object Reference") (OtherComp :type "PrimitiveComponent Object Reference") (OtherBodyIndex :type Integer) (bFromSweep :type Boolean) (SweepResult :type "HitResult Structure (by ref)"))
  (bind _asbp_bullet (cast `/Game/Weapons/BP_Bullet` OtherActor))
  (`/Game/ObjectPooling/PooledObject.ReturnToPool` _asbp_bullet)
  (bind _output_get (set `self.Lives` (- (`self.Lives`) 1)))
  (if (<= _output_get 0)
    (`self.K2_DestroyActor`)))

(event `self.ReceiveBeginPlay`
  (add `PrimitiveComponent.OnComponentBeginOverlap` (`self.DetectionArea`) (delegate `OnDetectionBeginOverlap`))
  (add `PrimitiveComponent.OnComponentBeginOverlap` (`self.EnemyArea`) (delegate `OnEnemyBeginOverlap`)))

(event `self.ReceiveActorEndOverlap`
  (params (OtherActor :type "Actor Object Reference"))
  (cast `/Game/ThirdPerson/Blueprints/BP_ThirdPersonCharacter` OtherActor)
  (`KismetSystemLibrary.K2_ClearAndInvalidateTimerHandle` (stale `OnDetectionBeginOverlap` _returnvalue)))

(event `OnDetectionBeginOverlap`
  (params (OverlappedComponent :type "PrimitiveComponent Object Reference") (OtherActor :type "Actor Object Reference") (OtherComp :type "PrimitiveComponent Object Reference") (OtherBodyIndex :type Integer) (bFromSweep :type Boolean) (SweepResult :type "HitResult Structure (by ref)"))
  (cast `/Game/ThirdPerson/Blueprints/BP_ThirdPersonCharacter` OtherActor)
  (bind _returnvalue (`KismetSystemLibrary.K2_SetTimerDelegate` (delegate `Shoot`) (`self.TimeToShoot`) true)))

(event `Shoot`
  (`/Game/ObjectPooling/ObjectPool.SpawnFromPool` (`self.LaserPool`) (`SceneComponent.K2_GetComponentToWorld` (`self.LaserPoint`))))

(fn `UserConstructionScript`)